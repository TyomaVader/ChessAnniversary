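; BP_FigureCharacter is a character Blueprint for a figure that belongs to a player, identified by a PlayerID.
; On BeginPlay it sets the first material slot of its mesh to a white board material for player zero and a black one for any other ID.
; A getter exposes the PlayerID to other code.
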(event `self.ReceiveBeginPlay`
  (`self.SetMeshColors`))

(fn `GetPlayerID`
  (returns (PlayerID :type Integer))
  (return (`self.PlayerID`)))

(fn `SetMeshColors`
  (if (== (`self.PlayerID`) 0)
    (`PrimitiveComponent.SetMaterial` (`self.Mesh`) 0 "/Game/Materials/Board_White.Board_White")
    (else
      (`PrimitiveComponent.SetMaterial` (`self.Mesh`) 0 "/Game/Materials/Board_Black.Board_Black"))))

(fn `UserConstructionScript`)
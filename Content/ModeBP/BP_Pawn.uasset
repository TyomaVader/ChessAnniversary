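; BP_Pawn seeds a placeholder test quest into its QuestManager on BeginPlay when no quests exist.
; It constructs a Trigger object, stores it as TestTrigger, and passes it into a single-step quest with test name and descriptions.
; An invalid trigger prints an error instead of adding the quest, and the construction script is empty.
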(event `self.ReceiveBeginPlay`
  (if (not (!= (`KismetArrayLibrary.Array_Length` (`QuestManager.Quests` (`self.QuestManager`))) 0))
    (bind _returnvalue (`|GenericCreateObject` "/Script/ChessDev.Trigger"))
    (bind _output_get (set `self.TestTrigger` _returnvalue))
    (if (`KismetSystemLibrary.IsValid` _output_get)
      (`QuestManager.AddQuest` (`self.QuestManager`) (make `QuestStruct` "TestName" "TestDescription" (`|MakeArray` (make `QuestStepStruct` "TestDescription" 0 _output_get) :!type "QuestStepStruct Structure")))
      (else
        (`KismetSystemLibrary.PrintText` "[ERROR] Trigger is invalid" true true (struct :`R` 1.0 :`B` 0.006945 :`A` 1.0))))))

(fn `UserConstructionScript`)
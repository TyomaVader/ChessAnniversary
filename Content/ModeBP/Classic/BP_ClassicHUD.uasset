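; BP_ClassicHUD is the Classic mode HUD that creates and manages the main HUD, pause menu and promotion widgets.
; BeginPlay adds all three to the viewport and registers both menus in WidgetList.
; Toggle events call ToggleWidget, which flips the target's visibility, collapses other listed menus, and on showing sets Game-and-UI input focused on it.
; Quest notifications bypass this list and go straight to the HUD widget.
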(event `self.ReceiveBeginPlay`
  ;[0 0 0] Game
  (bind _returnvalue (`|CreateWidget` "/Game/Widgets/WB_Classic_HUD.WB_Classic_HUD_C" (`self.GetOwningPlayerController`)))
  (bind _output_get (set `self.HUDWidget` _returnvalue))
  (`UserWidget.AddToViewport` _output_get 0)
  ;[0 0 0] GameMenus
  (bind _returnvalue_2 (`|CreateWidget` "/Game/Widgets/WB_PauseMenu.WB_PauseMenu_C" (`self.GetOwningPlayerController`)))
  (bind _output_get_2 (set `self.WB Game Menu` _returnvalue_2))
  (`KismetArrayLibrary.Array_Add` (`self.WidgetList`) _output_get_2)
  (bind _returnvalue_3 (`|CreateWidget` "/Game/Widgets/WB_PromotionWidget.WB_PromotionWidget_C" (`self.GetOwningPlayerController`)))
  (bind _output_get_3 (set `self.WB_PromotionWidget` _returnvalue_3))
  (`KismetArrayLibrary.Array_Add` (`self.WidgetList`) _output_get_3)
  (for _array_element (`self.WidgetList`)
    (`UserWidget.AddToViewport` _array_element 0)))

(event `TogglePromotionWidget`
  (`self.ToggleWidget` (`self.WB_PromotionWidget`)))

(event `ToggleNotificationWidget`
  (params (Title :type String) (NewProgress :type Integer) (TotalProgress :type Integer))
  (`/Game/Widgets/WB_Classic_HUD.ShowQuestNotification` (`self.HUDWidget`) (`KismetTextLibrary.Conv_StringToText` Title) NewProgress TotalProgress))

(event `TogglePauseMenu`
  (`self.ToggleWidget` (`self.WB Game Menu`)))

(fn `FocusWidget`
  (`Widget.SetVisibility` (`self.ActiveWidget`) "SelfHitTestInvisible")
  (`WidgetBlueprintLibrary.SetInputMode_GameAndUIEx` (`self.GetOwningPlayerController`) (`self.ActiveWidget`)))

(fn `ToggleWidget`
  (params (TargetWidget :type "UserWidget Object Reference"))
  (`/Engine/EditorBlueprintResources/StandardMacros.IsValid` TargetWidget
    (:`Is Valid`
      (set `self.ActiveWidget` (`local.TargetWidget`))
      (for _array_element (`self.WidgetList`)
        (`/Engine/EditorBlueprintResources/StandardMacros.IsValid` _array_element
          (:`Is Valid`
            (if (== (`self.ActiveWidget`) _array_element)
              (if (`Widget.IsVisible` (`self.ActiveWidget`))
                (`Widget.SetVisibility` (`self.ActiveWidget`) "Collapsed")
                (else
                  (`self.FocusWidget`)))
              (elif (`Widget.IsVisible` _array_element)
                (`Widget.SetVisibility` _array_element "Collapsed")))))))))

(fn `UserConstructionScript`)
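; Game mode for classic player-versus-AI chess, running the match through a spawned ChessEngine actor.
; On login it assigns the player ID, sets the standard starting position and begins the player's turn.
; CycleTurns submits the player's move to the engine, restarts the turn if rejected, otherwise mirrors it and the immediate AI reply on BP_Grid, checking for game end.
; Player starts are chosen from a lazily built map keyed by player ID.
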(event `self.K2_PostLogin`
  (params (NewPlayer :type "PlayerController Object Reference"))
  (`parent.K2_PostLogin` NewPlayer)
  (bind _returnvalue (`self.GetNumPlayers`))
  (bind _asbp_classic_pv_eplayer_controller (cast `/Game/ModeBP/Classic/BP_ClassicPvEPlayerController` NewPlayer))
  (`/Game/ModeBP/Classic/BP_ClassicPvEPlayerController.SetPlayerID` _asbp_classic_pv_eplayer_controller (- _returnvalue 1))
  (`self.StartGame`))

(event `StartGame`
  (`/Engine/EditorBlueprintResources/StandardMacros.IsValid` (`self.Engine`)
    (:`Is Valid`
      _)
    (:`Is Not Valid`
      (bind _returnvalue (`|SpawnActorFromClass` "/Script/ChessDev.ChessEngine" (`KismetMathLibrary.MakeTransform` (0.0 0.0 0.0)) "AlwaysSpawn" "MultiplyWithRoot" null null))
      (bind _output_get (set `self.Engine` _returnvalue))))
  (`ChessEngine.setBoardPosition` _output_get "rnbqkbnr/pppppppp/8/8/8/8/PPPPPPPP/RNBQKBNR" 255 true true true true 1.0)
  (bind _returnvalue_2 (`GameplayStatics.GetActorOfClass` "/Game/ModeBP/BP_Grid.BP_Grid_C"))
  (set `/Game/ModeBP/BP_Grid.GameMode` 0 _returnvalue_2)
  (`/Game/ModeBP/Classic/BP_ClassicPvEPlayerController.StartTurn` (`self.PlayerInTurn`)))

(event `CycleTurns`
  (bind _player_controller (`self.PlayerInTurn`))
  (bind _player_controller_2 (`self.PlayerInTurn`))
  (`/Game/ModeBP/Classic/BP_ClassicPvEPlayerController.EndTurn` (`self.PlayerInTurn`))
  (bind _returnvalue (`ChessEngine.makeMove` (`self.Engine`) (`/Game/ModeBP/Classic/BP_ClassicPvEPlayerController.fromTile` _player_controller_2) (`/Game/ModeBP/Classic/BP_ClassicPvEPlayerController.toTile` _player_controller_2) (`KismetMathLibrary.Conv_IntToByte` (`self.CurrentTurn`)) (`/Game/ModeBP/Classic/BP_ClassicPvEPlayerController.Figure Type` _player_controller_2)))
  (if _returnvalue
    (bind _returnvalue_2 (`GameplayStatics.GetActorOfClass` "/Game/ModeBP/BP_Grid.BP_Grid_C"))
    (`/Game/ModeBP/BP_Grid.PerformMove` _returnvalue_2 (`/Game/ModeBP/Classic/BP_ClassicPvEPlayerController.fromTile` _player_controller) (`/Game/ModeBP/Classic/BP_ClassicPvEPlayerController.toTile` _player_controller) (`/Game/ModeBP/Classic/BP_ClassicPvEPlayerController.Figure Type` _player_controller) false)
    (if (`ChessEngine.isGameFinished` (`self.Engine`))
      (`KismetSystemLibrary.PrintText` "Game Finished" true true (struct :`R` 1.0 :`B` 0.795438 :`A` 1.0))
      (else
        (bind (_from _to _promotionpiece) (`ChessEngine.makeAIMove` (`self.Engine`)))
        (`/Game/ModeBP/BP_Grid.PerformMove` _returnvalue_2 _from _to _promotionpiece false)
        (if (`ChessEngine.isGameFinished` (`self.Engine`))
          (`KismetSystemLibrary.PrintText` "Game Finished" true true (struct :`R` 1.0 :`B` 0.795438 :`A` 1.0))
          (else
            (set `self.CurrentTurn` 0)
            (`/Game/ModeBP/Classic/BP_ClassicPvEPlayerController.StartTurn` (`self.PlayerInTurn`))))))
    (else
      (`/Game/ModeBP/Classic/BP_ClassicPvEPlayerController.StartTurn` (`self.PlayerInTurn`)))))

(fn `ChoosePlayerStart`
  (params (Player :type "Controller Object Reference"))
  (returns (ReturnValue :type "Actor Object Reference"))
  (`self.InitSpawnPoints`)
  (bind _returnvalue (`self.GetNumPlayers`))
  (return (`BlueprintMapLibrary.Map_Find` (`self.SpawnPoints`) _returnvalue)))

(fn `InitSpawnPoints`
  (if (`BlueprintMapLibrary.Map_IsEmpty` (`self.SpawnPoints`))
    (bind _outactors (`GameplayStatics.GetAllActorsOfClass` "/Game/ModeBP/BP_PlayerStart.BP_PlayerStart_C"))
    (for _array_element _outactors
      (`BlueprintMapLibrary.Map_Add` (`self.SpawnPoints`) (`/Game/ModeBP/BP_PlayerStart.GetPlayerID` _array_element) _array_element))))

(fn `UserConstructionScript`)
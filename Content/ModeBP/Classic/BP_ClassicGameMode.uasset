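; Game mode for classic chess, running either player-versus-player or player-versus-AI matches.
; On login it assigns player IDs, hands triggers to quest managers and starts once the mode's player requirement is met.
; A spawned ChessEngine validates moves and detects game end, while BP_Grid performs accepted moves.
; CycleTurns alternates controllers or plays the AI reply and fires the first trigger; spawn points are mapped by player ID.
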(event `self.K2_PostLogin`
  (params (NewPlayer :type "PlayerController Object Reference"))
  ;[0 0 0] Initialize
  (`parent.K2_PostLogin` NewPlayer)
  (`self.CreateTriggers`)
  (bind _asbp_game_instance (cast `/Game/ModeBP/BP_GameInstance` (`GameplayStatics.GetGameInstance`)))
  (set `self.GameInstance` _asbp_game_instance)
  (bind _returnvalue (`self.GetNumPlayers`))
  (bind _asbp_classic_player_controller (cast `/Game/ModeBP/Classic/BP_ClassicPlayerController` NewPlayer))
  (`/Game/ModeBP/Classic/BP_ClassicPlayerController.SetPlayerID` _asbp_classic_player_controller (- _returnvalue 1))
  (`/Game/ModeBP/Classic/BP_ClassicPlayerController.LoadQuestManager` _asbp_classic_player_controller (`self.Triggers`))
  (switch `/Game/ModeBP/MainMenu/GameModes` (`/Game/ModeBP/BP_GameInstance.GameMode` (`self.GameInstance`))
    (:`NewEnumerator0`
      (bind _returnvalue_2 (`self.GetNumPlayers`))
      (if (== _returnvalue_2 2)
        (`self.StartGame`)
        (else
          (`KismetSystemLibrary.PrintText` "[ERROR] Not enough players!" true true (struct :`R` 1.0 :`A` 1.0)))))
    (:`NewEnumerator3`
      (`self.StartGame`))))

(event `StartGame`
  ;[0 0 0] Game Setup
  (bind _returnvalue (`|SpawnActorFromClass` "/Script/ChessDev.ChessEngine" (`KismetMathLibrary.MakeTransform` (0.0 0.0 0.0)) "AlwaysSpawn" "MultiplyWithRoot" null null))
  (bind _output_get (set `self.Engine` _returnvalue))
  (`ChessEngine.setBoardPosition` _output_get "rnbqkbnr/pppppppp/8/8/8/8/PPPPPPPP/RNBQKBNR" 255 true true true true 1.0)
  (`/Game/ModeBP/Classic/BP_ClassicPlayerController.StartTurn` (`self.PlayerInTurn`)))

(event `CycleTurns`
  (bind _player_controller (`self.PlayerInTurn`))
  (bind _player_controller_2 (`self.PlayerInTurn`))
  ;[0 0 0] Check Player Move
  (`/Game/ModeBP/Classic/BP_ClassicPlayerController.EndTurn` (`self.PlayerInTurn`))
  (bind _returnvalue (`ChessEngine.makeMove` (`self.Engine`) (`/Game/ModeBP/Classic/BP_ClassicPlayerController.fromTile` _player_controller_2) (`/Game/ModeBP/Classic/BP_ClassicPlayerController.toTile` _player_controller_2) (`KismetMathLibrary.Conv_IntToByte` (`self.CurrentTurn`)) (`/Game/ModeBP/Classic/BP_ClassicPlayerController.Figure Type` _player_controller_2)))
  (if _returnvalue
    (bind _returnvalue_2 (`GameplayStatics.GetActorOfClass` "/Game/ModeBP/BP_Grid.BP_Grid_C"))
    (`/Game/ModeBP/BP_Grid.PerformMove` _returnvalue_2 (`/Game/ModeBP/Classic/BP_ClassicPlayerController.fromTile` _player_controller) (`/Game/ModeBP/Classic/BP_ClassicPlayerController.toTile` _player_controller) (`/Game/ModeBP/Classic/BP_ClassicPlayerController.Figure Type` _player_controller) false)
    ;[0 0 0] Check If The Game Is Finished
    (if (`KismetMathLibrary.Conv_IntToBool` (`ChessEngine.isGameFinished` (`self.Engine`)))
      (`KismetSystemLibrary.PrintText` "Game Finished" true true (struct :`R` 1.0 :`B` 0.795438 :`A` 1.0))
      (else
        ;[0 0 0] Determine The Move Switch Model based on the Game Mode
        (switch `/Game/ModeBP/MainMenu/GameModes` (`/Game/ModeBP/BP_GameInstance.GameMode` (`self.GameInstance`))
          (:`NewEnumerator0`
            ;[0 0 0] Start The Other Player Move
            (set `self.CurrentTurn` (select `bool` (== (`self.CurrentTurn`) 0) :`true` 1))
            (`/Game/ModeBP/Classic/BP_ClassicPlayerController.StartTurn` (`self.PlayerInTurn`)))
          (:`NewEnumerator3`
            ;[0 0 0] Make The AI Move
            (bind (_from _to _promotionpiece) (`ChessEngine.makeAIMove` (`self.Engine`)))
            (`/Game/ModeBP/BP_Grid.PerformMove` _returnvalue_2 _from _to _promotionpiece false)
            (`Trigger.ActivateTrigger` (`|GetArrayItem` (`self.Triggers`)))
            ;[0 0 0] Check If The Game Is Finished
            (if (`KismetMathLibrary.Conv_IntToBool` (`ChessEngine.isGameFinished` (`self.Engine`)))
              (`KismetSystemLibrary.PrintText` "Game Finished" true true (struct :`R` 1.0 :`B` 0.795438 :`A` 1.0))
              (else
                ;[0 0 0] Get The Next Move From The Player
                (set `self.CurrentTurn` 0)
                (`/Game/ModeBP/Classic/BP_ClassicPlayerController.StartTurn` (`self.PlayerInTurn`))))))))
    (else
      (`/Game/ModeBP/Classic/BP_ClassicPlayerController.StartTurn` (`self.PlayerInTurn`)))))

(fn `ChoosePlayerStart`
  (params (Player :type "Controller Object Reference"))
  (returns (ReturnValue :type "Actor Object Reference"))
  (`self.InitSpawnPoints`)
  (bind _returnvalue (`self.GetNumPlayers`))
  (return (`BlueprintMapLibrary.Map_Find` (`self.SpawnPoints`) _returnvalue)))

(fn `CreateTriggers`
  (bind _returnvalue (`|GenericCreateObject` "/Script/ChessDev.Trigger"))
  (`KismetArrayLibrary.Array_Add` (`self.Triggers`) _returnvalue))

(fn `InitSpawnPoints`
  (if (`BlueprintMapLibrary.Map_IsEmpty` (`self.SpawnPoints`))
    (bind _outactors (`GameplayStatics.GetAllActorsOfClass` "/Game/ModeBP/BP_PlayerStart.BP_PlayerStart_C"))
    (for _array_element _outactors
      (`BlueprintMapLibrary.Map_Add` (`self.SpawnPoints`) (`/Game/ModeBP/BP_PlayerStart.GetPlayerID` _array_element) _array_element))))

(fn `UserConstructionScript`)
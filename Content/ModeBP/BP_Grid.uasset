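; Chess board actor that builds the tile grid, spawns pieces and tracks the board state for classic PvP, AI and CCG modes.
; Construction lays out instanced-mesh tiles and maps tile coordinates to transforms; on BeginPlay the authority spawns full armies, or only kings in CCG.
; Cursor traces resolve tiles, using a separate channel and dragged-card screen position in CCG.
; Moves teleport pieces, destroy captured ones, update the 64-slot array and handle promotion.
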(event `self.ReceiveBeginPlay`
  (bind _asbp_game_instance (cast `/Game/ModeBP/BP_GameInstance` (`GameplayStatics.GetGameInstance`)))
  (set `self.GameInstance` _asbp_game_instance)
  (if (`self.HasAuthority`)
    (`KismetArrayLibrary.Array_Resize` (`self.BoardState`) 64)
    (for _index (range 2)
      (switch `/Game/ModeBP/MainMenu/GameModes` (`/Game/ModeBP/BP_GameInstance.GameMode` (`self.GameInstance`))
        (:`NewEnumerator0`
          (`self.SpawnPawns` _index :!label _label)
          (`self.SpawnRooks` _index)
          (`self.SpawnKnights` _index)
          (`self.SpawnBishops` _index)
          (`self.SpawnKings` _index)
          (`self.SpawnQueens` _index))
        (:`NewEnumerator3`
          (goto _label))
        (:`NewEnumerator1`
          (`self.SpawnKings` _index))))))

(fn `AddPieceToBoardState`
  (params (Piece :type "/Game/ModeBP/BP_FigureCharacter Object Reference") (Tile :type "IntPoint Structure"))
  (`KismetArrayLibrary.Array_Set` (`self.BoardState`) (`self.TileToID` Tile) Piece))

(fn `GetCursorLocation`
  (params (PlayerIndex :type Integer))
  (returns (Location :type "Vector Structure"))
  (bind _returnvalue (`GameplayStatics.GetPlayerController` PlayerIndex))
  (bind (_worldlocation _worlddirection _returnvalue_2) (`PlayerController.DeprojectMousePositionToWorld` (`GameplayStatics.GetPlayerController` (`local.PlayerIndex`))))
  (bind (_worldlocation_2 _worlddirection_2) (`PlayerController.DeprojectMousePositionToWorld` (`GameplayStatics.GetPlayerController` (`local.PlayerIndex`))))
  (switch `/Game/ModeBP/MainMenu/GameModes` (`/Game/ModeBP/BP_GameInstance.GameMode` (`self.GameInstance`))
    (:`NewEnumerator0`
      _)
    (:`NewEnumerator3`
      _)
    (:`NewEnumerator1`
      (bind _asbp_ccgplayer_controller (cast `/Game/ModeBP/CCG/BP_CCGPlayerController` _returnvalue)
        (:`then`
          (if (and _returnvalue_2 (not (`/Game/ModeBP/CCG/BP_CCGPlayerController.isCardDragged` _asbp_ccgplayer_controller)))
            _
            (else
              (bind (_worldposition _worlddirection_3) (`GameplayStatics.DeprojectScreenToWorld` _returnvalue (`/Game/ModeBP/CCG/BP_CCGPlayerController.Pixel Position` _asbp_ccgplayer_controller)))
              (bind (_outhit _returnvalue_3) (`KismetSystemLibrary.LineTraceSingle` _worldposition (+ _worldposition (* _worlddirection_3 (10000.0 10000.0 10000.0))) "TraceTypeQuery3"))
              (if _returnvalue_3
                (return (+ (`.Location` (`GameplayStatics.BreakHitResult` _outhit)) (-70.0 -70.0 0.0)))
                (else
                  (return (-999.0 -999.0 -999.0)))))))
        (:`CastFailed`
          _))
      (bind (_outhit_2 _returnvalue_4) (`KismetSystemLibrary.LineTraceSingle` _worldlocation (+ _worldlocation (* _worlddirection (10000.0 10000.0 10000.0))) "TraceTypeQuery3"))
      (if _returnvalue_4
        (return (+ (`.Location` (`GameplayStatics.BreakHitResult` _outhit_2)) (-70.0 -70.0 0.0)))
        (else
          (return (-999.0 -999.0 -999.0))))))
  (bind (_outhit_3 _returnvalue_5) (`KismetSystemLibrary.LineTraceSingle` _worldlocation_2 (+ _worldlocation_2 (* _worlddirection_2 (10000.0 10000.0 10000.0))) "TraceTypeQuery1"))
  (if _returnvalue_5
    (return (+ (`.Location` (`GameplayStatics.BreakHitResult` _outhit_3)) (-70.0 -70.0 0.0)))
    (else
      (return (-999.0 -999.0 -999.0)))))

(fn `GetPieceAtTile`
  (params (Tile :type "IntPoint Structure"))
  (returns (Piece :type "/Game/ModeBP/BP_FigureCharacter Object Reference"))
  (return (`|GetArrayItem` (`self.BoardState`) (`self.TileToID` Tile))))

(fn `GetTileIDFromWorld`
  (params (Location :type "Vector Structure"))
  (returns (ID :type "IntPoint Structure"))
  (locals (LocationOnGrid :type "Vector Structure") (SnappedLocationOnGrid :type "Vector Structure" :default (0.0 0.0 0.0)))
  (set `local.LocationOnGrid` (- Location (`self.GridBottomLeftCorner`)))
  (set `local.SnappedLocationOnGrid` (`KismetMathLibrary.Vector_SnappedToGrid` (`local.LocationOnGrid`) 200.0))
  (return (`KismetMathLibrary.Conv_Vector2DToIntPoint` (`KismetMathLibrary.Conv_VectorToVector2D` (/ (`local.SnappedLocationOnGrid`) (`self.Tile Size`))))))

(fn `GetTileIDUnderCursor`
  (params (PlayerIndex :type Integer))
  (returns (ID :type "IntPoint Structure"))
  (locals (SelectedTileTransform :type "Transform Structure"))
  (bind _location (`self.GetCursorLocation` PlayerIndex))
  (bind _id (`self.GetTileIDFromWorld` _location))
  (return _id))

(fn `MovePieceBoardState`
  (params (FromTile :type "IntPoint Structure") (ToTile :type "IntPoint Structure"))
  (locals (PieceToMove :type "/Game/ModeBP/BP_FigureCharacter Object Reference"))
  (bind _piece (`self.GetPieceAtTile` FromTile))
  (set `local.PieceToMove` _piece)
  (`KismetArrayLibrary.Array_Set` (`self.BoardState`) (`self.TileToID` (`local.FromTile`)))
  (`KismetArrayLibrary.Array_Set` (`self.BoardState`) (`self.TileToID` (`local.ToTile`)) (`local.PieceToMove`)))

(fn `PerformMove`
  (params (FromTile :type "IntPoint Structure") (ToTile :type "IntPoint Structure") (PromotionType :type Byte) (IsCardSpawnMove :type Boolean))
  (locals (SelectedPiece :type "/Game/ModeBP/BP_FigureCharacter Object Reference") (DestinationPiece :type "/Game/ModeBP/BP_FigureCharacter Object Reference") (PromotionFigureType :type Byte))
  (bind _piece (`self.GetPieceAtTile` FromTile))
  (set `local.SelectedPiece` _piece)
  (bind _piece_2 (`self.GetPieceAtTile` ToTile))
  (set `local.DestinationPiece` _piece_2)
  (set `local.PromotionFigureType` PromotionType)
  (bind _selectedpiece (`local.SelectedPiece`)
    (:`then`
      (`self.K2_SetActorLocation` _selectedpiece (+ (.location (`BlueprintMapLibrary.Map_Find` (`self.TileTransforms`) (`local.ToTile`))) (100.0 100.0 50.0)) false true)
      (bind _destinationpiece (`local.DestinationPiece`)
        (:`then`
          (if (not (`local.IsCardSpawnMove`))
            (`self.K2_DestroyActor` _destinationpiece)))
        (:`else`
          _))
      (`self.MovePieceBoardState` (`local.FromTile`) (`local.ToTile`))
      (if (not (== (`local.PromotionFigureType`) 0))
        (`self.PromotePieceBoardState` (`local.PromotionFigureType`) (`local.ToTile`))))
    (:`else`
      (`KismetSystemLibrary.PrintText` "[ERROR] Invalid Piece Selected" true true (struct :`R` 1.0 :`A` 1.0)))))

(fn `PromotePieceBoardState`
  (params (PromotionFigureType :type Byte) (PromoteAtTile :type "IntPoint Structure"))
  (locals (NewType :type "/Game/ModeBP/BP_FigureCharacter Object Reference") (NewTranform :type "Transform Structure") (NewPlayerID :type Integer :default 0))
  (bind _piece (`self.GetPieceAtTile` PromoteAtTile))
  (set `local.NewTranform` (`self.GetTransform` _piece))
  (set `local.NewPlayerID` (`/Game/ModeBP/BP_FigureCharacter.PlayerID` _piece))
  (`self.K2_DestroyActor` _piece)
  (switch `int` (- (`KismetMathLibrary.Conv_ByteToInt` (`local.PromotionFigureType`)) 1)
    (:`Default`
      (`KismetSystemLibrary.PrintText` "[ERROR] Invalid promotion type" true true (struct :`R` 1.0 :`A` 1.0)))
    (:`0`
      (bind _returnvalue (`|SpawnActorFromClass` "/Game/Pieces/BP_KnightFigure.BP_KnightFigure_C" (`local.NewTranform`) "AlwaysSpawn" "MultiplyWithRoot" null (`local.NewPlayerID`) null))
      (set `local.NewType` _returnvalue)
      (`KismetArrayLibrary.Array_Set` (`self.BoardState`) (`self.TileToID` (`local.PromoteAtTile`)) (`local.NewType`) :!label _label))
    (:`1`
      (bind _returnvalue_2 (`|SpawnActorFromClass` "/Game/Pieces/BP_BishopFigure.BP_BishopFigure_C" (`local.NewTranform`) "AlwaysSpawn" "MultiplyWithRoot" null (`local.NewPlayerID`) null))
      (set `local.NewType` _returnvalue_2)
      (goto _label))
    (:`2`
      (bind _returnvalue_3 (`|SpawnActorFromClass` "/Game/Pieces/BP_RookFigure.BP_RookFigure_C" (`local.NewTranform`) "AlwaysSpawn" "MultiplyWithRoot" null (`local.NewPlayerID`) null))
      (set `local.NewType` _returnvalue_3)
      (goto _label))
    (:`3`
      (bind _returnvalue_4 (`|SpawnActorFromClass` "/Game/Pieces/BP_QueenFigure.BP_QueenFigure_C" (`local.NewTranform`) "AlwaysSpawn" "MultiplyWithRoot" null (`local.NewPlayerID`) null))
      (set `local.NewType` _returnvalue_4)
      (goto _label))))

(fn `SpawnBishops`
  (params (PlayerID :type Integer))
  (locals (Row :type Integer) (Col :type Integer))
  (set `local.Row` (select `int` (`local.PlayeriD`) :`0` 0 :`1` 7))
  (`|ExecutionSequence`
    (:`then_0`
      ;[1 1 1] Left
      (bind _output_get (set `local.Col` (select `int` (`local.PlayeriD`) :`0` 2 :`1` 5)))
      (bind _returnvalue (`|SpawnActorFromClass` "/Game/Pieces/BP_BishopFigure.BP_BishopFigure_C" (`KismetMathLibrary.MakeTransform` (+ (.location (`BlueprintMapLibrary.Map_Find` (`self.TileTransforms`) (make `IntPoint` (`local.Row`) _output_get))) (100.0 100.0 50.0))) "AlwaysSpawn" "MultiplyWithRoot" null (`local.PlayeriD`) null))
      (`self.AddPieceToBoardState` _returnvalue (make `IntPoint` (`local.Row`) (`local.Col`))))
    (:`then_1`
      ;[1 1 1] Right
      (bind _output_get_2 (set `local.Col` (select `int` (`local.PlayeriD`) :`0` 5 :`1` 2)))
      (bind _returnvalue_2 (`|SpawnActorFromClass` "/Game/Pieces/BP_BishopFigure.BP_BishopFigure_C" (`KismetMathLibrary.MakeTransform` (+ (.location (`BlueprintMapLibrary.Map_Find` (`self.TileTransforms`) (make `IntPoint` (`local.Row`) _output_get_2))) (100.0 100.0 50.0))) "AlwaysSpawn" "MultiplyWithRoot" null (`local.PlayeriD`) null))
      (`self.AddPieceToBoardState` _returnvalue_2 (make `IntPoint` (`local.Row`) (`local.Col`))))))

(fn `SpawnGrid`
  (params (SpawnLocationCenter :type "Vector Structure") (TileSize :type "Vector Structure") (GridSize :type "Vector2D Structure"))
  (locals (X :type Integer) (Y :type Integer) (TileTransform :type "Transform Structure"))
  (bind (_grid_size_x _grid_size_y) (`KismetMathLibrary.BreakVector2D` (`self.Grid Size`)))
  (bind _grid_size_x_2 (`KismetMathLibrary.BreakVector2D` (`self.Grid Size`)))
  (set `self.Spawn Location Center` SpawnLocationCenter)
  (set `self.Tile Size` TileSize)
  (set `self.Grid Size` GridSize)
  (`StaticMeshComponent.SetStaticMesh` (`self.HierarchicalInstancedStaticMesh`) null)
  (set `self.GridBottomLeftCorner` (- (`self.Spawn Location Center`) (* (/ (`self.Grid Size`) (2.0 2.0)) (`self.Tile Size`))))
  (for _index (range (`KismetMathLibrary.Round` _grid_size_x_2))
    (set `local.X` _index)
    (for _index_2 (range (`KismetMathLibrary.Round` _grid_size_y))
      (set `local.Y` _index_2)
      (bind _output_get (set `local.TileTransform` (`KismetMathLibrary.MakeTransform` (+ (`self.GridBottomLeftCorner`) (* (`self.Tile Size`) (`KismetMathLibrary.MakeVector` (`KismetMathLibrary.Conv_IntToDouble` (`local.X`)) (`KismetMathLibrary.Conv_IntToDouble` (`local.Y`))))) (struct) (/ (`self.Tile Size`) (200.0 200.0 7.0)))))
      (`BlueprintMapLibrary.Map_Add` (`self.TileTransforms`) (make `IntPoint` (`local.X`) (`local.Y`)) _output_get)
      (`InstancedStaticMeshComponent.AddInstance` (`self.HierarchicalInstancedStaticMesh`) (`local.TileTransform`) false))))

(fn `SpawnKings`
  (params (PlayerID :type Integer))
  (locals (Row :type Byte) (Col :type Byte))
  (set `local.Row` (`KismetMathLibrary.Conv_IntToByte` (select `int` (`local.PlayerID`) :`0` 0 :`1` 7)))
  (bind _output_get (set `local.Col` 4))
  (bind _returnvalue (`|SpawnActorFromClass` "/Game/Pieces/BP_KingFigure.BP_KingFigure_C" (`KismetMathLibrary.MakeTransform` (+ (.location (`BlueprintMapLibrary.Map_Find` (`self.TileTransforms`) (make `IntPoint` (`KismetMathLibrary.Conv_ByteToInt` (`local.Row`)) (`KismetMathLibrary.Conv_ByteToInt` _output_get)))) (100.0 100.0 50.0))) "Undefined" "OverrideRootScale" null (`local.PlayeriD`) null))
  (`self.AddPieceToBoardState` _returnvalue (make `IntPoint` (`KismetMathLibrary.Conv_ByteToInt` (`local.Row`)) (`KismetMathLibrary.Conv_ByteToInt` (`local.Col`)))))

(fn `SpawnKnights`
  (params (PlayerID :type Integer))
  (locals (Row :type Integer) (Col :type Integer))
  (set `local.Row` (select `int` (`local.PlayerID`) :`0` 0 :`1` 7))
  (`|ExecutionSequence`
    (:`then_0`
      ;[1 1 1] Left
      (bind _output_get (set `local.Col` (select `int` (`local.PlayeriD`) :`0` 1 :`1` 6)))
      (bind _returnvalue (`|SpawnActorFromClass` "/Game/Pieces/BP_KnightFigure.BP_KnightFigure_C" (`KismetMathLibrary.MakeTransform` (+ (.location (`BlueprintMapLibrary.Map_Find` (`self.TileTransforms`) (make `IntPoint` (`local.Row`) _output_get))) (100.0 100.0 50.0)) (select `int` (`local.PlayeriD`) :`0` (struct) :`1` (struct :`Yaw` 180.0) :!type "Rotator Structure")) "AlwaysSpawn" "MultiplyWithRoot" null (`local.PlayeriD`) null))
      (`self.AddPieceToBoardState` _returnvalue (make `IntPoint` (`local.Row`) (`local.Col`))))
    (:`then_1`
      ;[1 1 1] Right
      (bind _output_get_2 (set `local.Col` (select `int` (`local.PlayeriD`) :`0` 6 :`1` 1)))
      (bind _returnvalue_2 (`|SpawnActorFromClass` "/Game/Pieces/BP_KnightFigure.BP_KnightFigure_C" (`KismetMathLibrary.MakeTransform` (+ (.location (`BlueprintMapLibrary.Map_Find` (`self.TileTransforms`) (make `IntPoint` (`local.Row`) _output_get_2))) (100.0 100.0 50.0)) (select `int` (`local.PlayeriD`) :`0` (struct) :`1` (struct :`Yaw` 180.0) :!type "Rotator Structure")) "AlwaysSpawn" "MultiplyWithRoot" null (`local.PlayeriD`) null))
      (`self.AddPieceToBoardState` _returnvalue_2 (make `IntPoint` (`local.Row`) (`local.Col`))))))

(fn `SpawnPawns`
  (params (PlayerID :type Integer))
  (locals (Row :type Integer) (Col :type Integer))
  (bind _output_get (set `local.Row` (select `int` PlayerID :`0` 1 :`1` 6)))
  (for _index (range 8)
    (bind _output_get_2 (set `local.Col` _index))
    (bind _returnvalue (`|SpawnActorFromClass` "/Game/Pieces/BP_PawnFigure.BP_PawnFigure_C" (`KismetMathLibrary.MakeTransform` (+ (.location (`BlueprintMapLibrary.Map_Find` (`self.TileTransforms`) (make `IntPoint` _output_get _output_get_2))) (100.0 100.0 50.0))) "AlwaysSpawn" "MultiplyWithRoot" null (`local.PlayerID`) null))
    (`self.AddPieceToBoardState` _returnvalue (make `IntPoint` (`local.Row`) (`local.Col`)))))

(fn `SpawnPieceAtTile`
  (params (PlayerID :type Integer) (Tile :type "IntPoint Structure") (Figure :type "/Game/ModeBP/BP_FigureCharacter Class Reference"))
  (returns (SpawnedPiece :type "/Game/ModeBP/BP_FigureCharacter Object Reference"))
  (locals (Row :type Integer) (Col :type Integer))
  (bind (_tile_x _tile_y) (break `IntPoint` (`local.Tile`)))
  (bind _tile_x_2 (break `IntPoint` (`local.Tile`)))
  (bind _output_get (set `local.Row` _tile_x_2))
  (bind _output_get_2 (set `local.Col` _tile_y))
  (bind _returnvalue (`|SpawnActorFromClass` (`local.Figure`) (`KismetMathLibrary.MakeTransform` (+ (.location (`BlueprintMapLibrary.Map_Find` (`self.TileTransforms`) (make `IntPoint` _output_get _output_get_2))) (100.0 100.0 50.0))) "AlwaysSpawn" "MultiplyWithRoot" null (`local.PlayerID`) null))
  (`self.AddPieceToBoardState` _returnvalue (make `IntPoint` (`local.Row`) (`local.Col`)))
  (return _returnvalue))

(fn `SpawnQueens`
  (params (PlayerID :type Integer))
  (locals (Row :type Byte) (Col :type Byte))
  (set `local.Row` (`KismetMathLibrary.Conv_IntToByte` (select `int` (`local.PlayerID`) :`0` 0 :`1` 7)))
  (bind _output_get (set `local.Col` 3))
  (bind _returnvalue (`|SpawnActorFromClass` "/Game/Pieces/BP_QueenFigure.BP_QueenFigure_C" (`KismetMathLibrary.MakeTransform` (+ (.location (`BlueprintMapLibrary.Map_Find` (`self.TileTransforms`) (make `IntPoint` (`KismetMathLibrary.Conv_ByteToInt` (`local.Row`)) (`KismetMathLibrary.Conv_ByteToInt` _output_get)))) (100.0 100.0 50.0))) "Undefined" "OverrideRootScale" null (`local.PlayeriD`) null))
  (`self.AddPieceToBoardState` _returnvalue (make `IntPoint` (`KismetMathLibrary.Conv_ByteToInt` (`local.Row`)) (`KismetMathLibrary.Conv_ByteToInt` (`local.Col`)))))

(fn `SpawnRooks`
  (params (PlayeriD :type Integer))
  (locals (Row :type Integer) (Col :type Integer))
  (set `local.Row` (select `int` (`local.PlayeriD`) :`0` 0 :`1` 7))
  (`|ExecutionSequence`
    (:`then_0`
      ;[1 1 1] Left
      (bind _output_get (set `local.Col` (select `int` (`local.PlayeriD`) :`0` 0 :`1` 7)))
      (bind _returnvalue (`|SpawnActorFromClass` "/Game/Pieces/BP_RookFigure.BP_RookFigure_C" (`KismetMathLibrary.MakeTransform` (+ (.location (`BlueprintMapLibrary.Map_Find` (`self.TileTransforms`) (make `IntPoint` (`local.Row`) _output_get))) (100.0 100.0 50.0))) "AlwaysSpawn" "MultiplyWithRoot" null (`local.PlayeriD`) null))
      (`self.AddPieceToBoardState` _returnvalue (make `IntPoint` (`local.Row`) (`local.Col`))))
    (:`then_1`
      ;[1 1 1] Right
      (bind _output_get_2 (set `local.Col` (select `int` (`local.PlayeriD`) :`0` 7 :`1` 0)))
      (bind _returnvalue_2 (`|SpawnActorFromClass` "/Game/Pieces/BP_RookFigure.BP_RookFigure_C" (`KismetMathLibrary.MakeTransform` (+ (.location (`BlueprintMapLibrary.Map_Find` (`self.TileTransforms`) (make `IntPoint` (`local.Row`) _output_get_2))) (100.0 100.0 50.0))) "AlwaysSpawn" "MultiplyWithRoot" null (`local.PlayeriD`) null))
      (`self.AddPieceToBoardState` _returnvalue_2 (make `IntPoint` (`local.Row`) (`local.Col`))))))

(fn `UserConstructionScript`
  (`self.SpawnGrid` (`self.Spawn Location Center`) (`self.Tile Size`) (`self.Grid Size`)))